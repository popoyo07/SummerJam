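; BP_Camera_Switcher is a trigger actor that blends the player's view to a linked camera track while BP_ThirdPersonCharacter overlaps it.
; Entering saves the character's current track and, only if that track is valid, moves camera ownership to LinkTrack.
; Exiting blends back to the saved track, or to the character if none exists, and updates ownership.
; BeginPlay waits one tick, then switches for an already overlapping character.
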(event `self.ReceiveBeginPlay`
  (bind _overlappingactors (`self.GetOverlappingActors` "/Game/ThirdPerson/Blueprints/BP_ThirdPersonCharacter.BP_ThirdPersonCharacter_C"))
  (`KismetSystemLibrary.DelayUntilNextTick`)
  (if (`KismetArrayLibrary.Array_IsNotEmpty` _overlappingactors)
    (bind _asbp_third_person_character (cast `/Game/ThirdPerson/Blueprints/BP_ThirdPersonCharacter` (`|GetArrayItem` _overlappingactors)))
    (`self.SwitchToLinkedCam` _asbp_third_person_character)))

(event `self.ReceiveActorBeginOverlap`
  (params (OtherActor :type "Actor Object Reference"))
  (bind _asbp_third_person_character (cast `/Game/ThirdPerson/Blueprints/BP_ThirdPersonCharacter` OtherActor))
  (`self.SwitchToLinkedCam` _asbp_third_person_character))

(event `self.ReceiveActorEndOverlap`
  (params (OtherActor :type "Actor Object Reference"))
  (bind _asbp_third_person_character (cast `/Game/ThirdPerson/Blueprints/BP_ThirdPersonCharacter` OtherActor))
  (`self.SwitchToOldCam` _asbp_third_person_character))

(fn `SwitchToLinkedCam`
  (params (Character :type "/Game/ThirdPerson/Blueprints/BP_ThirdPersonCharacter Object Reference"))
  (bind _character (`local.Character`))
  (set `self.OldTrack` (`/Game/ThirdPerson/Blueprints/BP_ThirdPersonCharacter.CameraTrack` _character))
  (bind _asplayer_controller (cast `PlayerController` (`Pawn.GetController` _character)))
  (`PlayerController.SetViewTargetWithBlend` _asplayer_controller (`self.LinkTrack`) (`self.Blend Time`) "VTBlend_Cubic" 0.0 true)
  (bind _oldtrack (`self.OldTrack`)
    (:`then`
      (`/Game/Game/BluePrints/BP_CameraTrack.SetCamOwner` _oldtrack null)
      (`/Game/Game/BluePrints/BP_CameraTrack.SetCamOwner` (`self.LinkTrack`) (`local.Character`)))
    (:`else`)))

(fn `SwitchToOldCam`
  (params (Character :type "/Game/ThirdPerson/Blueprints/BP_ThirdPersonCharacter Object Reference"))
  (bind _asplayer_controller (cast `PlayerController` (`Pawn.GetController` (`local.Character`))))
  (bind _oldtrack (`self.OldTrack`)
    (:`then`
      (`PlayerController.SetViewTargetWithBlend` _asplayer_controller _oldtrack (`self.Blend Time`) "VTBlend_Cubic" 0.0 true)
      (`/Game/Game/BluePrints/BP_CameraTrack.SetCamOwner` (`self.LinkTrack`) null)
      (`/Game/Game/BluePrints/BP_CameraTrack.SetCamOwner` (`self.OldTrack`) (`local.Character`))
      (set `self.OldTrack` null))
    (:`else`
      (`PlayerController.SetViewTargetWithBlend` _asplayer_controller (`local.Character`) (`self.Blend Time`) "VTBlend_Cubic" 0.0 true)
      (`/Game/Game/BluePrints/BP_CameraTrack.SetCamOwner` (`self.LinkTrack`) null))))

(fn `UserConstructionScript`)