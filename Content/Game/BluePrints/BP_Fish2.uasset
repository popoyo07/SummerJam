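; BP_Fish2 is a clickable fish actor that wanders horizontally through the level.
; On begin play and on each arrival, RandomTarget picks a point MoveRadius away from the current location in a random XY direction.
; Tick eases the fish toward that target with VInterpTo, without sweeping.
; Clicking prints a debug message, destroys the fish and spawns a new BP_Fish2 at SpawnTransform.
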(event `self.ReceiveBeginPlay`
  (`self.RandomTarget`))

(event `self.ReceiveTick`
  (params (DeltaSeconds :type "Float (single-precision)"))
  (`self.K2_SetActorLocation` (`KismetMathLibrary.VInterpTo` (`self.K2_GetActorLocation`) (`self.Target`) DeltaSeconds 10.0))
  (if (< (`KismetMathLibrary.Vector_Distance` (`self.K2_GetActorLocation`) (`self.Target`)) 0.01)
    (`self.RandomTarget`)))

(event `self.ReceiveActorOnClicked`
  (params (ButtonPressed :type "Key Structure"))
  (`KismetSystemLibrary.PrintString` "fish is clicked")
  (`self.K2_DestroyActor`)
  (`|SpawnActorFromClass` "BP_Fish2_C" (`self.Spawn Transform`) "Undefined" "MultiplyWithRoot" null null))

(event `RandomTarget`
  (bind (_returnvalue_x _returnvalue_y) (`KismetMathLibrary.BreakVector` (`KismetMathLibrary.RandomUnitVector`)))
  (set `self.PreviousLocation` (`self.K2_GetActorLocation`))
  (set `self.Target` (+ (* (`KismetMathLibrary.Normal` (`KismetMathLibrary.MakeVector` _returnvalue_x _returnvalue_y)) (`self.MoveRadius`)) (`self.K2_GetActorLocation`))))

(fn `UserConstructionScript`)