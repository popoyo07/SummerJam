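; BP_TinCanTable is a tin can table that awards score through the third-person game mode when cans leave it.
; UpdateArray fills TinCansExist with the BP_TinCan actors overlapping the OnTableBox volume.
; When a can ends its overlap, it is removed from that array, and a successful removal calls IncrementCanScore on the game mode cached at BeginPlay, so only tracked cans score, once each.
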(event `self.ReceiveBeginPlay`
  (bind _asbp_third_person_game_mode (cast `/Game/ThirdPerson/Blueprints/BP_ThirdPersonGameMode` (`GameplayStatics.GetGameMode`)))
  (set `self.GameMode` _asbp_third_person_game_mode))

(event `self.OnTableBox.OnComponentEndOverlap`
  (params (OverlappedComponent :type "PrimitiveComponent Object Reference") (OtherActor :type "Actor Object Reference") (OtherComp :type "PrimitiveComponent Object Reference") (OtherBodyIndex :type Integer))
  (bind _asbp_tin_can (cast `/Game/Game/BluePrints/BP_TinCan` OtherActor))
  (bind _returnvalue (`KismetArrayLibrary.Array_RemoveItem` (stale `Update Array` _output_get) _asbp_tin_can))
  (if _returnvalue
    (`/Game/ThirdPerson/Blueprints/BP_ThirdPersonGameMode.Increment Can Score` (`self.GameMode`))))

(event `Update Array`
  (bind _output_get (set `self.TinCansExist` (`PrimitiveComponent.GetOverlappingActors` (`self.OnTableBox`) "/Game/Game/BluePrints/BP_TinCan.BP_TinCan_C"))))

(fn `UserConstructionScript`)