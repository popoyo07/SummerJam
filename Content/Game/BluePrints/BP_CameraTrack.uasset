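; BP_CameraTrack is a rail camera that follows its owning character along splines.
; Each tick it maps the spine_04 socket's nearest point on Path to a time, samples CmeraTrack there, and aims at the owner.
; Location and rotation ease in with separate lag speeds; SetCamOwner snaps the camera and toggles tick.
; Directional distance lag is inactive: LagDirection is computed, but the offset is forced to zero.
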(event `self.ReceiveTick`
  (params (DeltaSeconds :type "Float (single-precision)"))
  (bind _camowner (`self.CamOwner`)
    (:`then`
      (`self.UpdateCamera` (`SceneComponent.GetSocketLocation` (`Character.Mesh` _camowner) "spine_04"))
      (`self.InterpLocation`)
      (`self.InterpRotation`)
      (`self.UpdateMovementLagOffset`))
    (:`else`)))

(fn `GetTimeAlongSplineAtNearbyLocation`
  (params (WorldLocation :type "Vector Structure") (DistanceLag :type "Float (double-precision)"))
  (returns (ReturnValue :type "Float (single-precision)"))
  (bind _returnvalue (`SplineComponent.FindInputKeyClosestToWorldLocation` (`self.Path`) (`local.WorldLocation`)))
  (bind _returnvalue_2 (`self.GetVelocity` (`self.CamOwner`)))
  (set `self.LagDirection` (`KismetMathLibrary.SelectInt` (`KismetMathLibrary.SelectInt` 1 2 (== (`KismetMathLibrary.Conv_RotatorToVector` (`SplineComponent.GetRotationAtSplineInputKey` (`self.Path`) _returnvalue "World")) (`KismetMathLibrary.Normal` _returnvalue_2) :`ErrorTolerance` 1.0)) 0 (> (`KismetMathLibrary.VSize` (`KismetMathLibrary.MakeVector` (.x _returnvalue_2) (.y _returnvalue_2))) 300.0)))
  (return (`SplineComponent.GetTimeAtDistanceAlongSpline` (`self.Path`) (- (`SplineComponent.GetDistanceAlongSplineAtSplineInputKey` (`self.Path`) _returnvalue) (`local.DistanceLag`)))))

(fn `InterpLocation`
  (bind _returnvalue (`SceneComponent.K2_GetComponentLocation` (`self.Camera`)))
  (if (not (== (`self.DesiredLocation`) _returnvalue :`ErrorTolerance` 1.0))
    (`SceneComponent.K2_SetWorldLocation` (`self.Camera`) (`KismetMathLibrary.VInterpTo` _returnvalue (`self.DesiredLocation`) (`GameplayStatics.GetWorldDeltaSeconds`) (`self.MovementLagSpeed`)) false false)))

(fn `InterpRotation`
  (bind _returnvalue (`SceneComponent.K2_GetComponentRotation` (`self.Camera`)))
  (if (not (== (`self.DesiredRotation`) _returnvalue :`ErrorTolerance` 0.01))
    (`SceneComponent.K2_SetWorldRotation` (`self.Camera`) (`KismetMathLibrary.RInterpTo` _returnvalue (`self.DesiredRotation`) (`GameplayStatics.GetWorldDeltaSeconds`) (`self.RotationLagSppeed`)) false false)))

(fn `SetCamOwner`
  (params (Character :type "/Game/ThirdPerson/Blueprints/BP_ThirdPersonCharacter Object Reference"))
  (bind _output_get (set `self.CamOwner` Character))
  (`/Engine/EditorBlueprintResources/StandardMacros.IsValid` _output_get
    (:`Is Valid`
      (`self.SetActorTickEnabled` true)
      (`self.UpdateCamera` (`SceneComponent.GetSocketLocation` (`Character.Mesh` (`self.CamOwner`)) "spine_04"))
      (`SceneComponent.K2_SetWorldLocationAndRotation` (`self.Camera`) (`self.DesiredLocation`) (`self.DesiredRotation`) false false))
    (:`Is Not Valid`
      (`self.SetActorTickEnabled` false))))

(fn `UpdateCamera`
  (params (WorldLocation :type "Vector Structure"))
  (set `self.DesiredLocation` (`SplineComponent.GetLocationAtTime` (`self.CmeraTrack`) (`self.GetTimeAlongSplineAtNearbyLocation` WorldLocation (`self.MoevementOffset`)) "World" false))
  (set `self.DesiredRotation` (`KismetMathLibrary.FindLookAtRotation` (`SceneComponent.K2_GetComponentLocation` (`self.Camera`)) (`self.K2_GetActorLocation` (`self.CamOwner`)))))

(fn `UpdateMovementLagOffset`
  (set `self.MoevementOffset` 0.0))

(fn `UserConstructionScript`)