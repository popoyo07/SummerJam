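; BP_Sky is a day-night cycle that drives sun, moon and fog from a 24-hour clock.
; Tick advances Time by TimeDilation, wraps it at 24 and pins it to 225 when CycleOn is off.
; Time sets sun pitch, the opposite moon pitch, and fog density through a curve.
; Every update also finds all PointLight actors, lighting them after 12 and zeroing their intensity otherwise.
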(event `self.ReceiveTick`
  (params (DeltaSeconds :type "Float (single-precision)"))
  ; Setting/Resetting Time
  (bind _output_get (set `self.Time` (+ (* DeltaSeconds (`self.TimeDilation`)) (`self.Time`))))
  (if (>= _output_get 24.0)
    (set `self.Time` 0.0)
    (else
      (if (not (`self.CycleOn`))
        (set `self.Time` 225.0))
      ; Rotating Directional Light Sun
      (`SceneComponent.K2_SetRelativeRotation` (`self.DirectionalLight`) (`KismetMathLibrary.MakeRotator` 0.0 (* (/ (`self.Time`) 24.0) -360.0) 90.0) false false)
      (`|ExecutionSequence`
        (:`then_0`
          (if (> (`self.Time`) 12.0)
            (bind _outactors (`GameplayStatics.GetAllActorsOfClass` "/Script/Engine.PointLight"))
            (for _array_element _outactors
              (`LightComponent.SetIntensity` (`PointLight.PointLightComponent` _array_element) 92.083908))
            (else
              (bind _outactors_2 (`GameplayStatics.GetAllActorsOfClass` "/Script/Engine.PointLight"))
              (for _array_element_2 _outactors_2
                (`LightComponent.SetIntensity` (`PointLight.PointLightComponent` _array_element_2) 0.0)))))
        (:`then_1`
          ; Rotating Directional Light Moon
          (`SceneComponent.K2_SetRelativeRotation` (`self.DirectionalLight_Moon`) (`KismetMathLibrary.MakeRotator` 0.0 (+ (* (/ (`self.Time`) 24.0) -360.0) 180.0) 90.0) false false)
          ; Set Fog Density
          (`ExponentialHeightFogComponent.SetFogDensity` (`self.ExponentialHeightFog`) (`CurveFloat.GetFloatValue` (`self.FogDensityCurve`) (`self.Time`))))))))

(fn `UserConstructionScript`)