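; BP_Balloon is a balloon target that pops when hit by a dart and adds to the dart score.
; BeginPlay caches the BP_ThirdPersonGameMode reference.
; When a BP_Dart overlaps the capsule, the balloon destroys the dart, increments the score through the game mode, plays a sound at its location and destroys itself.
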(event `self.ReceiveBeginPlay`
  (bind _asbp_third_person_game_mode (cast `/Game/ThirdPerson/Blueprints/BP_ThirdPersonGameMode` (`GameplayStatics.GetGameMode`)))
  (set `self.GameMode` _asbp_third_person_game_mode))

(event `self.Capsule.OnComponentBeginOverlap`
  (params (OverlappedComponent :type "PrimitiveComponent Object Reference") (OtherActor :type "Actor Object Reference") (OtherComp :type "PrimitiveComponent Object Reference") (OtherBodyIndex :type Integer) (bFromSweep :type Boolean) (SweepResult :type "HitResult Structure (by ref)"))
  (if (`GameplayStatics.ObjectIsA` OtherActor "/Game/Game/BluePrints/BP_Dart.BP_Dart_C")
    ; Destroy the incoming dart
    (`self.K2_DestroyActor` OtherActor)
    (`/Game/ThirdPerson/Blueprints/BP_ThirdPersonGameMode.Increment Dart Score` (`self.GameMode`))
    (`GameplayStatics.PlaySoundAtLocation` "/Game/Game/Music/SFX/BallonSFX.BallonSFX" (`self.K2_GetActorLocation`) (struct) 1.0 1.0 0.0 null null null null)
    (`self.K2_DestroyActor`)))

(fn `UserConstructionScript`)